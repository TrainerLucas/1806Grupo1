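; BP_AutoJugador is the player-driven car, simulating a gearbox with CharacterMovement, controller-yaw steering, a vehicle UI, engine sound and a two-camera toggle.
; Boolean gear states step through Delay chains: up on throttle press, down when coasting or braking, with half gears while braking and reverse from standstill.
; A fast looping timer maps the gear to an acceleration rate, which Tick feeds into AddMovementInput.
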(event `Caja de cambios`
  ;[1 1 1] Caja de cambio
  (if (`self.Marcha 0`)
    (set `self.Marcha 0` false)
    (set `self.Marcha 1` true)
    (if (`self.Acelerar`)
      (`KismetSystemLibrary.Delay` 0.5)
      (set `self.Marcha 1` false :!label _label)
      (set `self.Marcha 2` true)
      (if (`self.Acelerar`)
        (`KismetSystemLibrary.Delay` 2.0)
        (set `self.Marcha 2` false :!label _label_2)
        (set `self.Marcha 3` true)
        (`KismetSystemLibrary.Delay` 3.0)
        (if (`self.Acelerar`)
          (set `self.Marcha 3` false :!label _label_3)
          (set `self.Marcha 4` true :!label _label_4)
          (`KismetSystemLibrary.Delay` 3.5)
          (if (`self.Acelerar`)
            (set `self.Marcha 4` false :!label _label_5)
            (set `self.Marcha 5` true :!label _label_6)))))
    (elif (`self.Marcha 1`)
      (goto _label)
      (elif (`self.Marcha 2`)
        (goto _label_2)
        (elif (`self.Marcha 3`)
          (goto _label_3)
          (elif (`self.Marcha 3,5`)
            (set `self.Marcha 3,5` false)
            (goto _label_4)
            (elif (`self.Marcha 4`)
              (goto _label_5)
              (elif (`self.Marcha 4,5`)
                (set `self.Marcha 4,5` false)
                (goto _label_6)))))))))

(event `Marcha atras/Freno`
  ;[1 1 1] Marcha atras
  (if (`self.Marcha Atras/Frenar`)
    (if (`self.Marcha 5`)
      (set `self.Marcha 5` false)
      (set `self.Marcha 4,5` true)
      (`KismetSystemLibrary.Delay` 0.2)
      (if (`self.Marcha Atras/Frenar`)
        (set `self.Marcha 4,5` false :!label _label_7)
        (set `self.Marcha 4` true)
        (`KismetSystemLibrary.Delay` 0.3)
        (if (`self.Marcha Atras/Frenar`)
          (set `self.Marcha 4` false :!label _label_8)
          (set `self.Marcha 3,5` true)
          (`KismetSystemLibrary.Delay` 0.5)
          (if (`self.Marcha Atras/Frenar`)
            (set `self.Marcha 3,5` false :!label _label_9)
            (set `self.Marcha 3` true)
            (`KismetSystemLibrary.Delay` 1.0)
            (if (`self.Marcha Atras/Frenar`)
              (set `self.Marcha 3` false :!label _label_10)
              (set `self.Marcha 2` true)
              (`KismetSystemLibrary.Delay` 1.5)
              (if (`self.Marcha Atras/Frenar`)
                (set `self.Marcha 2` false :!label _label_11)
                (set `self.Marcha 1` true)
                (`KismetSystemLibrary.Delay` 1.0)
                (if (`self.Marcha Atras/Frenar`)
                  (set `self.Marcha 1` false :!label _label_12)
                  (set `self.Marcha 0` true)
                  (if (`self.Marcha Atras/Frenar`)
                    (if (== (`KismetMathLibrary.VSize` (`MovementComponent.Velocity` (`self.CharacterMovement`))) 0.0)
                      (set `self.Marcha 0` false :!label _label_13)
                      (set `self.Marcha R` true)))))))))
      (elif (`self.Marcha 4,5`)
        (goto _label_7)
        (elif (`self.Marcha 4`)
          (goto _label_8)
          (elif (`self.Marcha 3,5`)
            (goto _label_9)
            (elif (`self.Marcha 3`)
              (goto _label_10)
              (elif (`self.Marcha 2`)
                (goto _label_11)
                (elif (`self.Marcha 1`)
                  (goto _label_12)
                  (elif (`self.Marcha 0`)
                    (goto _label_13)))))))))))

(event `Ajuste de velocidades`
  ;[1 1 1] Ajuste de velocidades
  (if (`self.Marcha 0`)
    (set `self.Tasa de aceleracion` 0.0)
    (elif (`self.Marcha 1`)
      (set `self.Tasa de aceleracion` 0.2)
      (elif (`self.Marcha 2`)
        (set `self.Tasa de aceleracion` 0.4)
        (elif (`self.Marcha 3`)
          (set `self.Tasa de aceleracion` 0.6)
          (elif (`self.Marcha 3,5`)
            (set `self.Tasa de aceleracion` 0.7)
            (elif (`self.Marcha 4`)
              (set `self.Tasa de aceleracion` 0.8)
              (elif (`self.Marcha 4,5`)
                (set `self.Tasa de aceleracion` 0.9)
                (elif (`self.Marcha 5`)
                  (set `self.Tasa de aceleracion` 1.0)
                  (elif (`self.Marcha R`)
                    (set `self.Tasa de aceleracion` -0.1)))))))))))

(event `self.ReceiveBeginPlay`
  ;[1 1 1] Begin play
  (`|ExecutionSequence`
    (:`then_0`
      (set `self.Marcha 0` true)
      (`KismetSystemLibrary.K2_SetTimerDelegate` (delegate `Ajuste de velocidades`) 0.001 true))
    (:`then_1`
      (bind _returnvalue (`|CreateWidget` "/Game/Autos/VehicleUI.VehicleUI_C"))
      (`UserWidget.AddToViewport` _returnvalue 0))))

(event `InputAction|Derecha`
  (params (Key :type "Key Structure"))
  ;[1 1 1] Input
  (:`Pressed`
    (set `self.Derecha` true))
  (:`Released`
    (set `self.Derecha` false)))

(event `InputAction|Acelerar`
  (params (Key :type "Key Structure"))
  ;[1 1 1] Input
  (:`Pressed`
    (set `self.Acelerar` true)
    (`|ExecutionSequence`
      (:`then_0`
        (`self.Caja de cambios`))
      (:`then_1`
        (bind _returnvalue (`GameplayStatics.SpawnSound2D` "/Game/Autos/Sonidos/Acelerar.Acelerar" 1.0 1.0 0.0 null))
        (set `self.NewVar_0` _returnvalue)
        (`AudioComponent.Play` (`self.NewVar_0`) 0.0))))
  (:`Released`
    (set `self.Acelerar` false)
    (`AudioComponent.StopDelayed` (`self.NewVar_0`) 1.2)))

(event `desaceleracion`
  ;[1 1 1] Desaceleracion
  (if (`self.Marcha Atras/Frenar`)
    _
    (elif (`self.Desacelerando`)
      (if (`self.Marcha 5`)
        (`KismetSystemLibrary.Delay` 1.0)
        (set `self.Marcha 5` false)
        (set `self.Marcha 4` true)
        (`KismetSystemLibrary.Delay` 4.0 :!label _label_14)
        (if (`self.Acelerar`)
          _
          (elif (not (`self.Marcha Atras/Frenar`))
            (set `self.Marcha 4` false)
            (set `self.Marcha 3` true)
            (`KismetSystemLibrary.Delay` 2.0 :!label _label_15)
            (if (`self.Acelerar`)
              _
              (elif (not (`self.Marcha Atras/Frenar`))
                (set `self.Marcha 3` false)
                (set `self.Marcha 2` true)
                (`KismetSystemLibrary.Delay` 1.5 :!label _label_16)
                (if (`self.Acelerar`)
                  _
                  (elif (not (`self.Marcha Atras/Frenar`))
                    (set `self.Marcha 2` false)
                    (set `self.Marcha 1` true)
                    (`KismetSystemLibrary.Delay` 0.2 :!label _label_17)
                    (if (`self.Acelerar`)
                      _
                      (elif (not (`self.Marcha Atras/Frenar`))
                        (set `self.Marcha 1` false)
                        (set `self.Marcha 0` true)))))))))
        (elif (`self.Marcha 4`)
          (goto _label_14)
          (elif (`self.Marcha 3`)
            (goto _label_15)
            (elif (`self.Marcha 2`)
              (goto _label_16)
              (elif (`self.Marcha 1`)
                (goto _label_17)))))))))

(event `InputAction|Marcha atras`
  (params (Key :type "Key Structure"))
  ;[1 1 1] Input
  (:`Pressed`
    (set `self.Marcha Atras/Frenar` true))
  (:`Released`
    (set `self.Marcha Atras/Frenar` false)))

(event `InputAction|Izquierda`
  (params (Key :type "Key Structure"))
  ;[1 1 1] Input
  (:`Pressed`
    (set `self.Izquierda` true))
  (:`Released`
    (set `self.Izquierda` false)))

(event `Key|C`
  (params (Key :type "Key Structure"))
  ;[1 1 1] Tipo de camara
  (:`Pressed`
    (`/Engine/EditorBlueprintResources/StandardMacros.FlipFlop`
      (:`A`
        (`self.Camara tp`))
      (:`B`
        (`self.Camara fp`)))))

(event `self.ReceiveTick`
  (params (DeltaSeconds :type "Float (single-precision)"))
  ;[1 1 1] Event tick
  (`|ExecutionSequence`
    (:`then_0`
      (if (`self.Acelerar`)
        (set `self.Desacelerando` false :!label _label_18)
        ;[1 1 1] Acelerar
        (`self.AddMovementInput` (`self.GetActorForwardVector`) (+ (`self.Velocidad minima`) (`self.Tasa de aceleracion`)))
        (elif (`self.Marcha Atras/Frenar`)
          (goto _label_18)
          (else
            (set `self.Desacelerando` true)))))
    (:`then_1`
      ;[1 1 1] Derecha
      (if (`self.Derecha`)
        (`self.AddControllerYawInput` (+ DeltaSeconds (`self.Tasa de girar`)))))
    (:`then_2`
      ;[1 1 1] Izquierda
      (if (`self.Izquierda`)
        (`self.AddControllerYawInput` (- DeltaSeconds (`self.Tasa de girar`)))))
    (:`then_3`
      (if (`self.Desacelerando`)
        (`self.desaceleracion`)))
    (:`then_4`
      ;[1 1 1] Marcha atras activar
      (if (`self.Marcha Atras/Frenar`)
        (`self.Marcha atras/Freno`)
        (elif (`self.Marcha R`)
          (set `self.Marcha R` false)
          (set `self.Marcha 0` true))))
    (:`then_5`
      (if true
        _))))

(fn `Camara fp`
  (`ActorComponent.Deactivate` (`self.Camera1`))
  (`ActorComponent.Activate` (`self.Camera`) false))

(fn `Camara tp`
  (`ActorComponent.Deactivate` (`self.Camera`))
  (`ActorComponent.Activate` (`self.Camera1`) false))

(fn `UserConstructionScript`)